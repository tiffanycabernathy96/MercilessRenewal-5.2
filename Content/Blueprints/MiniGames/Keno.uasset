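; Keno minigame logic that draws winning numbers and decides how many chickens the player wins.
; GenerateWinningNumbers picks ten random numbers without repeats by removing each pick from a temporary copy of the number pool.
; DetermineNumberOfChickensWon is a hard-coded payout table mapping numbers played (one to five) and hit count to a reward of up to three chickens.
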(fn `DetermineNumberOfChickensWon`
  (params (NumberOfPlayerNumbers :type Integer) (NumberOfHits :type Integer))
  (returns (WonChickens :type Integer))
  (switch `int` NumberOfPlayerNumbers
    (:`1`
      (if (== NumberOfHits 1)
        _
        (else
          (return 0))))
    (:`2`
      (switch `int` NumberOfHits
        (:`0`
          (return 0))
        (:`1`
          _)
        (:`2`
          _)))
    (:`3`
      (switch `int` NumberOfHits
        (:`0`
          (return 0))
        (:`1`
          (return 0))
        (:`2`
          _)
        (:`3`
          (return 2))))
    (:`4`
      (switch `int` NumberOfHits
        (:`0`
          (return 0))
        (:`1`
          (return 0))
        (:`2`
          _)
        (:`3`
          (return 2))
        (:`4`
          (return 3))))
    (:`5`
      (switch `int` NumberOfHits
        (:`0`
          (return 0))
        (:`1`
          (return 0))
        (:`2`
          _)
        (:`3`
          _)
        (:`4`
          (return 2))
        (:`5`
          (return 3)))))
  (return 1))

(fn `GenerateWinningNumbers`
  (returns (ChoosenNumbers :type "Array of Integer"))
  (locals (GeneratedNumbers :type "Array of Integer") (AllPossibleNumbers :type "Array of Integer") (TempNumbers :type "Array of Integer") (HandIndex :type Integer))
  (set `local.TempNumbers` (`local.AllPossibleNumbers`))
  (for _ (range 10)
    (bind _output_get (set `local.HandIndex` (`KismetMathLibrary.RandomIntegerInRange` 0 (- (`KismetArrayLibrary.Array_Length` (`local.TempNumbers`)) 1))))
    (`KismetArrayLibrary.Array_Add` (`local.GeneratedNumbers`) (`|GetArrayItem` (`local.TempNumbers`) _output_get))
    (`KismetArrayLibrary.Array_Remove` (`local.TempNumbers`) _output_get))
  (return (`local.GeneratedNumbers`)))