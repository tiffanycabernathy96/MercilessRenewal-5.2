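; Blackjack minigame rules for a player against an NPC, with cards stored as numeric values.
; GeneratePlayersHands deals both hands into one array, player's first, then draws for the NPC until 17 or a natural blackjack.
; Hit draws a random remaining card and flags busts, counting aces as 1.
; DetermineWinner counts one ace as 11 when possible, but adds only 1 for all aces otherwise; ties lose for the player.
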(fn `DetermineWinner`
  (params (PlayerHand :type "Array of Integer") (NPCHand :type "Array of Integer"))
  (returns (PlayerWon :type Boolean))
  (locals (PlayerSum :type Integer) (AltPlayerSum :type Integer) (NPCSum :type Integer) (AltNPCSum :type Integer) (PlayerEndSum :type Integer) (NPCEndSum :type Integer) (PlayersValuesSet :type Boolean) (NPCValuesSet :type Boolean) (numAces :type Integer) (NewLocalVar_0 :type Integer))
  (bind _playersum (`local.PlayerSum`))
  (bind _npcsum (`local.NPCSum`))
  (bind _playersum_2 (`local.PlayerSum`))
  (bind _playersum_3 (`local.PlayerSum`))
  (bind _playersum_4 (`local.PlayerSum`))
  (bind _playersum_5 (`local.PlayerSum`))
  (bind _npcsum_2 (`local.NPCSum`))
  (bind _npcsum_3 (`local.NPCSum`))
  (bind _npcsum_4 (`local.NPCSum`))
  (bind _npcsum_5 (`local.NPCSum`))
  ;[1 1 1] Determine Who Won
  (set `local.numAces` 0)
  (set `local.PlayerSum` 0)
  (set `local.AltPlayerSum` 0)
  (for _array_element PlayerHand
    (if (== _array_element 1)
      (set `local.numAces` (+ (`local.numAces`) 1))
      (else
        (set `local.PlayerSum` (+ (`local.PlayerSum`) _array_element)))))
  (switch `int` (`local.numAces`)
    (:`0`
      _)
    (:`1`
      (if (<= (+ (`local.PlayerSum`) 11) 21)
        (set `local.PlayerSum` (+ _playersum_2 11))
        (else
          (set `local.PlayerSum` (+ _playersum_2 1)))))
    (:`2`
      (if (<= (+ (`local.PlayerSum`) 12) 21)
        (set `local.PlayerSum` (+ _playersum_3 12))
        (else
          (set `local.PlayerSum` (+ _playersum_3 1)))))
    (:`3`
      (if (<= (+ (`local.PlayerSum`) 13) 21)
        (set `local.PlayerSum` (+ _playersum_4 13))
        (else
          (set `local.PlayerSum` (+ _playersum_4 1)))))
    (:`4`
      (if (<= (+ (`local.PlayerSum`) 14) 21)
        (set `local.PlayerSum` (+ _playersum_5 14))
        (else
          (set `local.PlayerSum` (+ _playersum_5 1))))))
  (if (> (`local.PlayerSum`) 21)
    (return false)
    (else
      (set `local.numAces` 0)
      (for _array_element_2 NPCHand
        (if (== _array_element_2 1)
          (set `local.numAces` (+ (`local.numAces`) 1))
          (else
            (set `local.NPCSum` (+ (`local.NPCSum`) _array_element_2)))))
      (switch `int` (`local.numAces`)
        (:`0`
          _)
        (:`1`
          (if (<= (+ (`local.NPCSum`) 11) 21)
            (set `local.NPCSum` (+ _npcsum_4 11))
            (else
              (set `local.NPCSum` (+ _npcsum_4 1)))))
        (:`2`
          (if (<= (+ (`local.NPCSum`) 12) 21)
            (set `local.NPCSum` (+ _npcsum_3 12))
            (else
              (set `local.NPCSum` (+ _npcsum_3 1)))))
        (:`3`
          (if (<= (+ (`local.NPCSum`) 13) 21)
            (set `local.NPCSum` (+ _npcsum_2 13))
            (else
              (set `local.NPCSum` (+ _npcsum_2 1)))))
        (:`4`
          (if (<= (+ (`local.NPCSum`) 14) 21)
            (set `local.NPCSum` (+ _npcsum_5 14))
            (else
              (set `local.NPCSum` (+ _npcsum_5 1))))))
      (if (> (`local.NPCSum`) 21)
        (return true)
        (else
          (if (== _playersum _npcsum)
            _
            (elif (> _playersum _npcsum)
              (return true)
              (else
                _)))
          (return false))))))

(fn `GeneratePlayersHands`
  (returns (GeneratedHands :type "Array of Integer") (RemainingDeck :type "Array of Integer") (NPCBust :type Boolean))
  (locals (Deck :type "Array of Integer") (TempDeck :type "Array of Integer") (GeneratedHand :type "Array of Integer") (HandIndex :type Integer) (NPCBusted :type Boolean) (NPCHandSum :type Integer))
  (bind _generatedhand (`local.GeneratedHand`))
  (bind _output (`|GetArrayItem` _generatedhand 3))
  (bind _output_2 (`|GetArrayItem` _generatedhand 2))
  (bind _returnvalue (`KismetMathLibrary.RandomIntegerInRange` 0 (- (`KismetArrayLibrary.Array_Length` (`local.TempDeck`)) 1)))
  ;[1 1 1] Generate the first two cards for both players and remaining cards for NPC as needed
  (set `local.TempDeck` (`local.Deck`))
  (for _ (range 4)
    (bind _output_get (set `local.HandIndex` _returnvalue))
    (`KismetArrayLibrary.Array_Add` (`local.GeneratedHand`) (`|GetArrayItem` (`local.TempDeck`) _output_get))
    (`KismetArrayLibrary.Array_Remove` (`local.TempDeck`) _output_get))
  (for _index (range 2 (`KismetArrayLibrary.Array_Length` _generatedhand)) :!label _label
    (bind _output_get_2 (set `local.NPCHandSum` (+ (`local.NPCHandSum`) (`|GetArrayItem` (`local.GeneratedHand`) _index)))))
  (if (or (>= _output_get_2 17) (or (and (== _output_2 10) (== _output 1)) (and (== _output_2 1) (== _output 10))))
    (if (> _output_get_2 21)
      (set `local.NPCBusted` true)
      (else
        (set `local.NPCBusted` false)))
    (return (`local.GeneratedHand`) (`local.TempDeck`) (`local.NPCBusted`))
    (else
      (bind _output_get_3 (set `local.HandIndex` _returnvalue))
      (`KismetArrayLibrary.Array_Add` (`local.GeneratedHand`) (`|GetArrayItem` (`local.TempDeck`) _output_get_3))
      (`KismetArrayLibrary.Array_Remove` (`local.TempDeck`) _output_get_3)
      (set `local.NPCHandSum` 0)
      (goto _label))))

(fn `Hit`
  (params (RemainingDeck :type "Array of Integer") (PlayersHand :type "Array of Integer"))
  (returns (NewCardDrawn :type Integer) (NewRemainingDeck :type "Array of Integer") (PlayerBust :type Boolean))
  (locals (TempDeck :type "Array of Integer") (PlayerSum :type Integer) (PlayerBusted :type Boolean) (IndexChoosen :type Integer))
  ;[1 1 1] The player has decided to take another card
  (bind _output_get (set `local.TempDeck` RemainingDeck))
  (bind _output_get_2 (set `local.IndexChoosen` (`KismetMathLibrary.RandomIntegerInRange` 0 (- (`KismetArrayLibrary.Array_Length` RemainingDeck) 1))))
  (`KismetArrayLibrary.Array_Remove` _output_get _output_get_2)
  (for _array_element PlayersHand
    (set `local.PlayerSum` (+ _array_element (`local.PlayerSum`))))
  (bind _output (`|GetArrayItem` RemainingDeck _output_get_2))
  (if (> (+ (`local.PlayerSum`) _output) 21)
    (set `local.PlayerBusted` true)
    (else
      (set `local.PlayerBusted` false)))
  (return _output (`local.TempDeck`) (`local.PlayerBusted`)))