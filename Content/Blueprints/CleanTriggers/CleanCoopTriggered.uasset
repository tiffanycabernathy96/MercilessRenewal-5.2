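; CleanCoopTriggered is a trigger actor that shows the HUD's clean box prompt for the coop.
; Begin overlap reveals the box only for a FirstPersonCharacter with a CoopLevel above zero.
; End overlap hides it for any actor, without a cast or level check.
; Both events find the HUD through GetAllWidgetsOfClass and set ShowCleanBox on the first result.
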(event `self.ReceiveActorBeginOverlap`
  (params (OtherActor :type "Actor Object Reference"))
  (bind _asfirst_person_character (cast `/Game/FirstPersonBP/Blueprints/FirstPersonCharacter` OtherActor))
  (if (> (`/Game/FirstPersonBP/Blueprints/FirstPersonCharacter.CoopLevel` _asfirst_person_character) 0)
    (bind _foundwidgets (`WidgetBlueprintLibrary.GetAllWidgetsOfClass` "/Game/Blueprints/HUD.HUD_C"))
    (set `/Game/Blueprints/HUD.ShowCleanBox` "Visible" (`|GetArrayItem` _foundwidgets))))

(event `self.ReceiveActorEndOverlap`
  (params (OtherActor :type "Actor Object Reference"))
  (bind _foundwidgets (`WidgetBlueprintLibrary.GetAllWidgetsOfClass` "/Game/Blueprints/HUD.HUD_C"))
  (set `/Game/Blueprints/HUD.ShowCleanBox` "Hidden" (`|GetArrayItem` _foundwidgets)))

(fn `UserConstructionScript`)