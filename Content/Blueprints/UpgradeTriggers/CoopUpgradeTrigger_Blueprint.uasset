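; Trigger actor that shows the HUD interaction prompt for a Coop upgrade while the coop level is below 2.
; On BeginPlay it caches the first HUD widget, whose Character reference supplies the CoopLevel checked on overlap, without checking the overlapping actor.
; A valid overlap shows the interaction box and sets IsOverlapping; ending overlap hides the box but leaves the flag set.
; The upgrade itself is not handled here.
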(event `self.ReceiveBeginPlay`
  (bind _foundwidgets (`WidgetBlueprintLibrary.GetAllWidgetsOfClass` "/Game/Blueprints/HUD.HUD_C" false))
  (set `self.HUD` (`|GetArrayItem` _foundwidgets)))

(event `self.ReceiveActorBeginOverlap`
  (params (OtherActor :type "Actor Object Reference"))
  (bind _ashud (cast `/Game/Blueprints/HUD` (`self.HUD`)))
  (bind _asfirst_person_character (cast `/Game/FirstPersonBP/Blueprints/FirstPersonCharacter` (`/Game/Blueprints/HUD.Character` _ashud)))
  (if (< (`/Game/FirstPersonBP/Blueprints/FirstPersonCharacter.CoopLevel` _asfirst_person_character) 2)
    (set `/Game/Blueprints/HUD.ShowInteractionBox` "Visible" _ashud)
    (set `self.isOverlapping` true)))

(event `self.ReceiveActorEndOverlap`
  (params (OtherActor :type "Actor Object Reference"))
  (bind _ashud (cast `/Game/Blueprints/HUD` (`self.HUD`)))
  (set `/Game/Blueprints/HUD.ShowInteractionBox` "Hidden" _ashud))

(fn `UserConstructionScript`)